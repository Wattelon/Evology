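; AR player pawn that opens the main menu on start and lets a touch place a creature on tracked real-world geometry.
; A touch first runs a world object trace; if nothing is hit, it traces tracked AR objects and spawns BP_Creature at the first hit.
; After spawning, it shows the EvoStart widget with UI-only input.
; Tick debug-draws all tracked geometry.
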(event EventBeginPlay
  (Input|SetInputModeUIOnly (Game|GetPlayerController 0) 0 "DoNotLock")
  (bind _returnvalue (UserInterface|CreateWidget "/Game/Blueprints/MainMenu.MainMenu_C"))
  (bind _output_get (Variables|Default|SetMainMenu _returnvalue))
  (UserInterface|Viewport|AddtoViewport _output_get 0))

(event EventTick
  (params (DeltaSeconds :type Float%20%28single-precision%29))
  (bind _returnvalue (Class|ARBlueprintLibrary|GetAllGeometries))
  (for _array_element _returnvalue
    (Class|ARBlueprintLibrary|DebugDrawTrackedGeometry _array_element "(R=0.020808,G=0.593750,B=0.000000,A=0.750000)")))

(event Input|TouchEvents|InputTouch
  (params (Location :type Vector) (FingerIndex :type ETouchIndex%20Enum))
  (bind _returnvalue (Game|GetPlayerController 0))
  (bind _returnvalue_2 (Game|GetPlayerController 0))
  (bind (_locationx _locationy) (Class|PlayerController|GetInputTouchState _returnvalue_2 "Touch1"))
  (bind _returnvalue_3 (Math|Vector2D|MakeVector2D _locationx _locationy))
  (:Pressed
    (bind _returnvalue_4 (CallFunction|WorldHitTest _returnvalue_3))
    (if (not _returnvalue_4)
      (bind _returnvalue_5 (Class|ARBlueprintLibrary|LineTraceTrackedObjects _returnvalue_3 false false))
      (Math|Integer|CompareInt (Utilities|Array|Length _returnvalue_5)
        (:>
          (bind _returnvalue_6 (Game|SpawnActorfromClass "/Game/Blueprints/BP_Creature.BP_Creature_C" (Class|ARTraceResultLibrary|GetLocaltoWorldTransform (Utilities|Array|Get(acopy) _returnvalue_5)) "AlwaysSpawn" 0 0))
          (Variables|Default|SetBPCreatureRef _returnvalue_6)
          (bind _returnvalue_7 (UserInterface|CreateWidget "/Game/Blueprints/EvoStart.EvoStart_C" _returnvalue))
          (UserInterface|Viewport|AddtoViewport _returnvalue_7 0)
          (Input|SetInputModeUIOnly _returnvalue _returnvalue_7 "DoNotLock"))))))

(fn ConstructionScript)

(fn WorldHitTest
  (params (ScreenPosition :type Vector%202D%20Structure%20%28by%20ref%29))
  (bind _returnvalue (Game|GetPlayerController 0))
  (bind (_worldposition _worlddirection) (Class|GameplayStatics|DeprojectScreentoWorld _returnvalue ScreenPosition))
  (bind (_outhits _returnvalue_2) (Class|KismetSystemLibrary|LineTraceMultiforObjects _worldposition (+ _worldposition (* _worlddirection 1000)) (Utilities|Array|MakeArray "ObjectTypeQuery1" "ObjectTypeQuery2" "ObjectTypeQuery3" "ObjectTypeQuery4" "ObjectTypeQuery5" "ObjectTypeQuery6") false 0 "None" true))
  (return _outhits _returnvalue_2))